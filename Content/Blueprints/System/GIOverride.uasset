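; GIOverride forces the world map to load with the FML_GM game mode by reopening it through a console command.
; Init waits, reads the level name once, then enters a delayed polling loop that rechecks that stored name.
; On MAP_TheWorld or its DLC variant, a DoOnce gate opens MAP_TheWorld with a game override and calls Retry.
; Other level names reset the gate and keep the loop running.
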(event Custom|Retry
  (if (or (Utilities|Enum|Equal(Enum) (stale EventInit _returnvalue) "MAP_TheWorld") (Utilities|Enum|Equal(Enum) (stale EventInit _returnvalue) "MAP_TheWorld_DLC")) :!label _label
    (Utilities|FlowControl|DoOnce false :!label _label_2
      (:Completed
        (Utilities|FlowControl|Delay 3.0)
        (Development|ExecuteConsoleCommand "open MAP_TheWorld?game=/Game/Blueprints/System/GameModes/FML_GM.FML_GM_C" (Game|GetPlayerController 0))
        (CallFunction|Retry)))
    (else
      (Utilities|FlowControl|Delay 3.0)
      (Utilities|FlowControl|Sequence
        (:then_0
          (goto _label_2 Reset))
        (:then_1
          (goto _label))))))

(event EventInit
  (Utilities|FlowControl|Delay 1e+01)
  (bind _returnvalue (Game|GetCurrentLevelName true))
  (if (or (Utilities|Enum|Equal(Enum) _returnvalue "MAP_TheWorld") (Utilities|Enum|Equal(Enum) _returnvalue "MAP_TheWorld_DLC")) :!label _label
    (Utilities|FlowControl|DoOnce false :!label _label_2
      (:Completed
        (Utilities|FlowControl|Delay 3.0)
        (Development|ExecuteConsoleCommand "open MAP_TheWorld?game=/Game/Blueprints/System/GameModes/FML_GM.FML_GM_C" (Game|GetPlayerController 0))
        (CallFunction|Retry)))
    (else
      (Utilities|FlowControl|Delay 3.0)
      (Utilities|FlowControl|Sequence
        (:then_0
          (goto _label_2 Reset))
        (:then_1
          (goto _label))))))