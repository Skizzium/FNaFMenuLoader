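; Blueprint stamina component that adds a developer UI hotkey and leaves stamina behavior to its parent class.
; Tick calls the parent, then polls the X key on player controller 0 and calls OnToggleDevUI on the FNAFBasePlayerController.
; A DoOnce, reset while the key is up, limits this to one toggle per press.
; BeginPlay and GetStaminaPercentage simply forward to the parent.
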(event EventBeginPlay
  (|CallParentFunction))

(event EventTick
  (params (DeltaSeconds :type Float%20%28single-precision%29))
  (Utilities|FlowControl|Sequence
    (:then_0
      (|CallParentFunction DeltaSeconds))
    (:then_1
      (if (Game|Player|IsInputKeyDown (Game|GetPlayerController 0) "X")
        (Utilities|FlowControl|DoOnce false :!label _label
          (:Completed
            (bind _asfnafbase_player_controller (Utilities|Casting|CastToFNAFBasePlayerController (Game|GetPlayerController 0)))
            (Class|FNAFBasePlayerController|OnToggleDevUI _asfnafbase_player_controller)))
        (else
          (goto _label Reset))))))

(fn GetStaminaPercentage
  (return (|CallParentFunction)))